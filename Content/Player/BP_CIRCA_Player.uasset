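; BP_CIRCA_Player is a viewer pawn that follows a Possessed target's replicated VR camera in desktop or VR mode.
; BeginPlay creates the CIRCA player UI, links it to the in-world VR widget, and binds its VR and rotation-control events.
; EnableVR swaps viewport and world widgets, toggles the HMD and movement, and resets rotation.
; Tick matches the full camera transform on desktop, but only location in VR; Enhanced Input drives playback and target switching.
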(event `self.ReceiveBeginPlay`
  (bind _returnvalue (`GameplayStatics.GetPlayerController` 0))
  (`EnhancedInputSubsystemInterface.AddMappingContext` (pcsubsystem `EnhancedInputLocalPlayerSubsystem` _returnvalue) "/CIRCA/Inputs/MC_CIRCA_Player.MC_CIRCA_Player" 0 (struct))
  (`WidgetBlueprintLibrary.SetInputMode_GameAndUIEx` _returnvalue null)
  (set `PlayerController.bShowMouseCursor` true _returnvalue)
  (`PlayerController.SetViewTargetWithBlend` _returnvalue self 0.0 "VTBlend_Linear" 0.0 false)
  (bind _returnvalue_2 (`|CreateWidget` "/CIRCA/UI/UW_CIRCA_Player.UW_CIRCA_Player_C" _returnvalue))
  (bind _output_get (set `self.Player` _returnvalue_2))
  (bind _asuw_circa_vr (cast `/CIRCA/UI/UW_CIRCA_VR` (`WidgetComponent.GetWidget` (`self.Widget`))))
  (`/CIRCA/UI/UW_CIRCA_Player.SetVRWidget` _output_get _asuw_circa_vr)
  (set `/CIRCA/UI/UW_CIRCA_VR.Player` _output_get _asuw_circa_vr)
  (`SceneComponent.SetVisibility` (`self.Widget`) false false)
  (`UserWidget.AddToViewport` (`self.Player`) 0)
  (add `/CIRCA/UI/UW_CIRCA_Player.EnableVR` (`self.Player`) (delegate `Enable VR`))
  (add `/CIRCA/UI/UW_CIRCA_Player.ControlRotation` (`self.Player`) (delegate `ControlRotation`))
  (if (`HeadMountedDisplayFunctionLibrary.IsHeadMountedDisplayEnabled`)
    (`/CIRCA/UI/UW_CIRCA_Player.ManualToggleDesktop` (`self.Player`))))

(event `Enable VR`
  (params (Enable :type Boolean))
  (`|ExecutionSequence`
    (:`then_0`
      (if Enable
        (`WidgetLayoutLibrary.RemoveAllWidgets`)
        (else
          (`UserWidget.AddToViewport` (`self.Player`) 0))))
    (:`then_1`
      (`SceneComponent.SetVisibility` (`self.Widget`) Enable false)
      (`HeadMountedDisplayFunctionLibrary.EnableHMD` Enable)
      (`Controller.SetControlRotation` (`GameplayStatics.GetPlayerController` 0) (`KismetMathLibrary.MakeRotator` 0.0))
      (`self.K2_SetActorTransform` (`KismetMathLibrary.MakeTransform` (0.0 0.0 0.0)) false true)
      (`ActorComponent.SetActive` (`self.MovementComponent`) (not Enable) true))
    (:`then_2`
      (set `self.VRMode` Enable)
      (`self.UpdateRotation`))))

(event `self.ReceiveTick`
  (params (DeltaSeconds :type "Float (single-precision)"))
  (bind _possessed (`self.Possessed`))
  (bind _returnvalue (`SceneComponent.K2_GetComponentToWorld` (`VRBaseCharacter.VRReplicatedCamera` _possessed)))
  (`/Engine/EditorBlueprintResources/StandardMacros.IsValid` _possessed
    (:`Is Valid`
      (if (`self.VRMode`)
        (`self.K2_SetActorLocation` (- (.location _returnvalue) (`SceneComponent.RelativeLocation` (`self.Camera`))) false true)
        (else
          (`SceneComponent.K2_SetWorldTransform` (`self.Camera`) _returnvalue false true))))))

(event `EnhancedInput|/CIRCA/Inputs/IA_CIRCA_PlayPause`
  (params (ActionValue :type Boolean) (ElapsedSeconds :type "Float (double-precision)") (TriggeredSeconds :type "Float (double-precision)") (InputAction :type "InputAction Object Reference" :default "/CIRCA/Inputs/IA_CIRCA_PlayPause.IA_CIRCA_PlayPause"))
  (:`Triggered`
    (`/CIRCA/UI/UW_CIRCA_Player.ManualTogglePlay` (`self.Player`))))

(event `ControlRotation`
  (params (control :type Boolean))
  (set `self.ShouldRotate` control)
  (`self.UpdateRotation`))

(event `EnhancedInput|/CIRCA/Inputs/IA_CIRCA_Previous`
  (params (ActionValue :type Boolean) (ElapsedSeconds :type "Float (double-precision)") (TriggeredSeconds :type "Float (double-precision)") (InputAction :type "InputAction Object Reference" :default "/CIRCA/Inputs/IA_CIRCA_Previous.IA_CIRCA_Previous"))
  (:`Triggered`
    (`/CIRCA/UI/UW_CIRCA_Player.ManualPossessPrevious` (`self.Player`))))

(event `EnhancedInput|/CIRCA/Inputs/IA_CRICA_Next`
  (params (ActionValue :type Boolean) (ElapsedSeconds :type "Float (double-precision)") (TriggeredSeconds :type "Float (double-precision)") (InputAction :type "InputAction Object Reference" :default "/CIRCA/Inputs/IA_CRICA_Next.IA_CRICA_Next"))
  (:`Triggered`
    (`/CIRCA/UI/UW_CIRCA_Player.ManualPossessNext` (`self.Player`))))

(event `EnhancedInput|/CIRCA/Inputs/IA_CIRCA_ShowHide`
  (params (ActionValue :type Boolean) (ElapsedSeconds :type "Float (double-precision)") (TriggeredSeconds :type "Float (double-precision)") (InputAction :type "InputAction Object Reference" :default "/CIRCA/Inputs/IA_CIRCA_ShowHide.IA_CIRCA_ShowHide"))
  (:`Triggered`
    (bind _isa (`/Engine/EditorBlueprintResources/StandardMacros.FlipFlop`)
      (:`A`
        _)
      (:`B`
        _))
    (`SceneComponent.SetVisibility` (`self.Widget`) (not _isa) false)))

(event `EnhancedInput|/CIRCA/Inputs/IA_CIRCA_Exit`
  (params (ActionValue :type Boolean) (ElapsedSeconds :type "Float (double-precision)") (TriggeredSeconds :type "Float (double-precision)") (InputAction :type "InputAction Object Reference" :default "/CIRCA/Inputs/IA_CIRCA_Exit.IA_CIRCA_Exit"))
  (:`Triggered`
    (`/CIRCA/UI/UW_CIRCA_Player.ManualToggleDesktop` (`self.Player`))))

(event `EnhancedInput|/CIRCA/Inputs/IA_CIRCA_Restart`
  (params (ActionValue :type Boolean) (ElapsedSeconds :type "Float (double-precision)") (TriggeredSeconds :type "Float (double-precision)") (InputAction :type "InputAction Object Reference" :default "/CIRCA/Inputs/IA_CIRCA_Restart.IA_CIRCA_Restart"))
  (:`Triggered`
    (`/CIRCA/UI/UW_CIRCA_Player.Restart` (`self.Player`))))

(fn `Possess`)

(fn `UpdateRotation`
  (set `CameraComponent.bUsePawnControlRotation` (and (not (`self.VRMode`)) (`self.ShouldRotate`)) (`self.Camera`)))

(fn `UserConstructionScript`)