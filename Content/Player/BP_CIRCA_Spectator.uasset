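; BP_CIRCA_Spectator is a player spectator Blueprint that starts and stops CIRCA recordings from debug keys.
; On BeginPlay it enables input for the local viewing controller and prints an on-screen prompt.
; R calls the StartRecording dispatcher and E calls StopRecording, each printing a status message.
; Two DoOnce gates reset each other so starts and stops alternate, allowing repeated takes.
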(event EventBeginPlay
  (Input|EnableInput (Pawn|GetLocalViewingPlayerController))
  (Development|PrintString "CIRCA: Press R to record" true true "(R=1.000000,G=0.000000,B=0.474510,A=1.000000)" 1e+01 "CIRCA"))

(event Collision|EventActorBeginOverlap
  (params (OtherActor :type Actor%20Object%20Reference)))

(event EventTick
  (params (DeltaSeconds :type Float%20%28single-precision%29)))

(event Input|KeyboardEvents|DebugKeyR
  (params (Key :type Key%20Structure :default "None") (ActionValue :type Input%20Action%20Value%20Structure))
  (:Pressed
    (Development|PrintString "CIRCA: Recording, press E to end the recording" true true "(R=1.000000,G=0.000000,B=0.474510,A=1.000000)" 2e+01 "CIRCA")
    (Utilities|FlowControl|DoOnce false
      (:Completed
        (Utilities|FlowControl|Sequence
          (:then_0
            (Utilities|FlowControl|DoOnce true) ; enters at Reset
          )
          (:then_1
            (Default|CallStartRecording)))))))

(event Input|KeyboardEvents|DebugKeyE
  (params (Key :type Key%20Structure :default "None") (ActionValue :type Input%20Action%20Value%20Structure))
  (:Pressed
    (Development|PrintString "CIRCA: Ended, press R to record another take" true true "(R=1.000000,G=0.000000,B=0.474510,A=1.000000)" 2e+01 "CIRCA")
    (Utilities|FlowControl|DoOnce true
      (:Completed
        (Utilities|FlowControl|Sequence
          (:then_0
            (Utilities|FlowControl|DoOnce false) ; enters at Reset
          )
          (:then_1
            (Default|CallStopRecording)))))))

(fn ConstructionScript)