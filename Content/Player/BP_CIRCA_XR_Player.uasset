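; BP_CIRCA_XR_Player is an XR player Blueprint that shows a laser while its widget interaction component points at menus.
; Each Tick checks for a hit-testable widget under the pointer, using two cross-resetting DoOnce gates to toggle the Niagara laser's visibility only on changes.
; While over a widget, it writes the laser's start and end points into the Niagara User.PointArray.
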(event `self.ReceiveTick`
  (params (DeltaSeconds :type "Float (single-precision)"))
  (bind _widgetinteraction (`self.WidgetInteraction`))
  (bind _ns_menulaser (`self.NS_MenuLaser`))
  (bind (_returnvalue_bblockinghit _returnvalue_binitialoverlap _returnvalue_time _returnvalue_distance _returnvalue_location _returnvalue_impactpoint) (`GameplayStatics.BreakHitResult` (`WidgetInteractionComponent.GetLastHitResult` _widgetinteraction)))
  (`parent.ReceiveTick` DeltaSeconds)
  (if (`WidgetInteractionComponent.IsOverHitTestVisibleWidget` _widgetinteraction)
    (`|ExecutionSequence`
      (:`then_0`
        (`/Engine/EditorBlueprintResources/StandardMacros.DoOnce` false :!label _label
          (:`Completed`
            (`SceneComponent.SetVisibility` (`self.NS_MenuLaser`) true false)
            (goto _label_2 :!via `Reset`))))
      (:`then_1`
        (`NiagaraDataInterfaceArrayFunctionLibrary.SetNiagaraArrayVectorValue` _ns_menulaser "User.PointArray" 0 (`SceneComponent.K2_GetComponentLocation` _widgetinteraction)) ; MenuLaser start location
        (`NiagaraDataInterfaceArrayFunctionLibrary.SetNiagaraArrayVectorValue` _ns_menulaser "User.PointArray" 1 _returnvalue_impactpoint) ; MenuLaser end location
      ))
    (else
      (`|ExecutionSequence`
        (:`then_0`
          (`/Engine/EditorBlueprintResources/StandardMacros.DoOnce` false :!label _label_2
            (:`Completed`
              (`SceneComponent.SetVisibility` (`self.NS_MenuLaser`) false false)
              (goto _label :!via `Reset`))))))))

(fn `UserConstructionScript`
  (`parent.UserConstructionScript`))