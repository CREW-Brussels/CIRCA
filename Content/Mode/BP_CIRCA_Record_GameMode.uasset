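; BP_CIRCA_Record_GameMode is a game mode that keeps a registry of actors with CIRCA components, apparently for recording.
; Component begin and end play events add or remove the owning actor in CIRCARecorded, without duplicates, and broadcast matching dispatchers when membership changes.
; HandleStartingNewPlayer runs the parent's start logic only for nonzero controller IDs, so player 0 skips default startup.
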(event `self.HandleStartingNewPlayer`
  (params (NewPlayer :type "PlayerController Object Reference"))
  (if (!= (`GameplayStatics.GetPlayerControllerID` NewPlayer) 0)
    (`parent.HandleStartingNewPlayer` NewPlayer)))

(event `CIRCA Component BeginPlay`
  (params (Component :type "/CIRCA/Component/CIRCA_Recorded Object Reference"))
  (bind _returnvalue (`ActorComponent.GetOwner` Component))
  (bind _circa_recorded (`self.CIRCA Recorded`))
  (if (not (`BlueprintSetLibrary.Set_Contains` _circa_recorded _returnvalue))
    (`BlueprintSetLibrary.Set_Add` _circa_recorded _returnvalue)
    (`self.On BeginPlay CIRCA Actor` _returnvalue)))

(event `CIRCA Component EndPlay`
  (params (Component :type "/CIRCA/Component/CIRCA_Recorded Object Reference"))
  (bind _returnvalue (`ActorComponent.GetOwner` Component))
  (bind _returnvalue_2 (`BlueprintSetLibrary.Set_Remove` (`self.CIRCA Recorded`) _returnvalue))
  (if _returnvalue_2
    (`self.On EndPlay CIRCA Actor` _returnvalue)))

(fn `UserConstructionScript`)